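; Game instance that keeps the player's best score persistent between play sessions.
; On Init it loads a BP_SaveGame from a fixed slot and restores the highest score, or creates a new save object if none exists.
; SaveBestScore stores the passed score as the score sum and, when it beats the record, updates the save, writes it to the slot and prints it.
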(event Custom|SaveBestScore
  (params (CurrentScore :type Float%20%28double-precision%29))
  (bind _savegame (Variables|Default|GetSaveGame))
  (Class|UWGameInstance|SetScoreSum CurrentScore)
  (if (> (Class|UWGameInstance|GetScoreSum) (Class|UWGameInstance|GetHighestScore))
    (Class|UWGameInstance|SetHighestScore (Class|UWGameInstance|GetScoreSum))
    (bind _output_get (Variables|/Game/Game/BP_SaveGame.BP_SaveGame_C|SetBestScore _savegame (Class|UWGameInstance|GetHighestScore)))
    (SaveGame|SaveGametoSlot _savegame (Variables|Default|GetSlot0))
    (Development|PrintString (Utilities|String|ToString(Float) _output_get))))

(event EventInit
  (bind _returnvalue (SaveGame|DoesSaveGameExist (Variables|Default|GetSlot0)))
  (if _returnvalue
    (bind _returnvalue_2 (SaveGame|LoadGamefromSlot (Variables|Default|GetSlot0)))
    (bind _asbp_save_game (Utilities|Casting|CastToBP_SaveGame _returnvalue_2))
    (bind _output_get (Variables|Default|SetSaveGame _asbp_save_game))
    (Class|UWGameInstance|SetHighestScore (Variables|/Game/Game/BP_SaveGame.BP_SaveGame_C|GetBestScore _output_get))
    (else
      (bind _returnvalue_3 (SaveGame|CreateSaveGameObject "/Game/Game/BP_SaveGame.BP_SaveGame_C"))
      (Variables|Default|SetSaveGame _returnvalue_3))))